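; BP_PlayerController is the player controller that owns the main HUD widget and bridges its chat UI to the game state.
; On BeginPlay, the local controller creates WB_MainWidget; pressing P focuses its chat text box and shows the chat background.
; SendChatMessageToServer posts the message with the sender's player state to the game state's BPChatComponent.
; SetFocusToTheGame restores game-only input and hides the chat background.
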(event `self.ReceiveBeginPlay`
  (if (`self.IsLocalController`)
    (bind _returnvalue (`|CreateWidget` "/Game/Widgets/WB_MainWidget.WB_MainWidget_C" self))
    (set `self.MainWidgetReference` _returnvalue)
    (`UserWidget.AddToViewport` _returnvalue 1)))

(event `Key|P`
  (params (Key :type "Key Structure"))
  (bind _wb_chat (`/Game/Widgets/WB_MainWidget.WB_Chat` (`self.MainWidgetReference`)))
  (:`Pressed`
    (`Widget.SetKeyboardFocus` (`/Game/Widgets/WB_Chat_SendMessagePanel.EditableTextBox_WriteMessage` (`/Game/Widgets/WB_Chat.WB_MessagePanelInsideChat` _wb_chat)))
    (`/Game/Widgets/WB_Chat.Toggle Chat Background` _wb_chat true)))

(event `SendChatMessageToServer`
  (params (Message :type Text))
  (`/Game/Blueprints/BP_ChatComponent.Post Message` (`/Game/Blueprints/BP_GameState.BP_ChatComponent` (cast `/Game/Blueprints/BP_GameState` (`GameplayStatics.GetGameState`) :!pure true)) Message (cast `/Game/Blueprints/BP_PlayerState` (`self.PlayerState`) :!pure true)))

(event `SetFocusToTheGame`
  (`WidgetBlueprintLibrary.SetInputMode_GameOnly` self)
  (`/Game/Widgets/WB_Chat.Toggle Chat Background` (`/Game/Widgets/WB_MainWidget.WB_Chat` (`self.MainWidgetReference`)) false))

(fn `UserConstructionScript`)